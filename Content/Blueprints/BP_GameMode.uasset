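; BP_GameMode is the game mode that runs the HUD, the end-of-game menu and quitting.
; On BeginPlay it focuses the viewport and shows WBP_HUD; Escape quits the game.
; Death and win events set MenuDescription, then share one path that pauses the game and shows WBP_Menu with a cursor.
; The menu's click event reopens "Level", removes the menu, hides the cursor and unpauses.
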(event `Key|Escape`
  (params (Key :type "Key Structure"))
  ;[1 1 1] Quit
  (:`Pressed`
    (`KismetSystemLibrary.QuitGame` null "Quit")))

(event `self.ReceiveBeginPlay`
  ;[1 1 1] HUD
  (`WidgetBlueprintLibrary.SetFocusToGameViewport`)
  (bind _returnvalue (`|CreateWidget` "/Game/Blueprints/WBP_HUD.WBP_HUD_C" (`GameplayStatics.GetPlayerControllerFromID` 0)))
  (bind _output_get (set `self.HUDWidget` _returnvalue))
  (`UserWidget.AddToViewport` _output_get 0))

(event `self.DieCharacterEvent`
  (bind _returnvalue (`GameplayStatics.GetPlayerController` 0))
  ;[1 1 1] Menu
  (set `self.MenuDescription` "You died!")
  (`GameplayStatics.SetGamePaused` true :!label _label)
  (bind _returnvalue_2 (`|CreateWidget` "/Game/Blueprints/WBP_Menu.WBP_Menu_C" _returnvalue))
  (set `PlayerController.bShowMouseCursor` true _returnvalue)
  (`UserWidget.AddToViewport` _returnvalue_2 0)
  (add `/Game/Blueprints/WBP_Menu.MenuClick` _returnvalue_2 (delegate `Event Menu Click`)))

(event `self.WinEvent`
  ;[1 1 1] Menu
  (set `self.MenuDescription` "You won!")
  (goto _label))

(event `Event Menu Click`
  ;[1 1 1] Menu
  (`GameplayStatics.OpenLevel` "Level")
  (`Widget.RemoveFromParent` (stale `self.DieCharacterEvent` _returnvalue_2))
  (set `PlayerController.bShowMouseCursor` false (`GameplayStatics.GetPlayerController` 0))
  (`GameplayStatics.SetGamePaused` false))

(fn `UserConstructionScript`)